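; HUD Blueprint that draws the shooter's crosshair on screen.
; On each DrawHUD it finds the screen center, raises that point 50 pixels, then subtracts the crosshair half-width and half-height variables to position a fixed-size crosshair texture.
; All other events and the construction script are empty.
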(event EventBeginPlay)

(event Collision|EventActorBeginOverlap
  (params (OtherActor :type Actor%20Object%20Reference)))

(event EventTick
  (params (DeltaSeconds :type Float%20%28single-precision%29)))

(event EventDrawHUD
  (params (SizeX :type Integer) (SizeY :type Integer))
  (Variables|Default|SetScreenCenter (Math|Vector2D|MakeVector2D (Math|Conversions|ToFloat(Integer) (/ SizeX 2)) (Math|Conversions|ToFloat(Integer) (/ SizeY 2))))
  (Variables|Default|SetCrosshairLocation (Math|Vector2D|MakeVector2D (.X (Math|Vector2D|BreakVector2D (Variables|Default|GetScreenCenter))) (- (.Y (Math|Vector2D|BreakVector2D (Variables|Default|GetScreenCenter))) 5e+01)))
  (Canvas|DrawTexture "/Game/_Game/Assets/Textures/Crosshairs/Cross_Q_9.Cross_Q_9" (- (.X (Math|Vector2D|BreakVector2D (Variables|Default|GetCrosshairLocation))) (Variables|Default|GetCrosshairHalfWidth)) (- (.Y (Math|Vector2D|BreakVector2D (Variables|Default|GetCrosshairLocation))) (Variables|Default|GetCrosshairHalfHeeight)) 64.0 64.0 0.0 0.0 1.0 1.0 "(R=1.000000,G=1.000000,B=1.000000,A=1.000000)"))

(fn ConstructionScript)